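; F-35B fighter vehicle Blueprint that turns flight and system inputs into visual animation and effects.
; Setter events drive control surfaces, cockpit controls, gear, canopy, bomb bay and refuel through its Anim Blueprint.
; Throttle and afterburner size the exhaust nozzles, which scale the Niagara jet plume.
; VTOL angle opens or closes fan shafts via a reversible timeline, while dust effects blend between conventional and VTOL emitters.
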(event `self.ReceiveBeginPlay`
  (`parent.ReceiveBeginPlay`)
  ;[1 1 1] Sets ABP Instances References
  (bind _asbpa_west_fighter_f35b (cast `/Game/VigilanteMovement/Vehicles/West_Fighter_F35B/BPA_West_Fighter_F35B` (`SkeletalMeshComponent.GetAnimInstance` (`self.SkeletalMesh`))))
  (set `self.AnimInstance` _asbpa_west_fighter_f35b)
  ;[1 1 1] Initial Exhaust and afterburner Settings
  (`self.SetExhaustNozzles` 0.6)
  (`NiagaraComponent.SetVariableVec3` (`self.NS_Jet`) "JetScale" (0.6 0.1 0.1))
  (`NiagaraComponent.SetVariableVec3` (`self.NS_Jet`) "JetRingsScale" (10.0 10.0 11.0))
  (`FXSystemComponent.SetFloatParameter` (`self.NS_Jet`) "Opacity divide" 1.0)
  (`self.SetAfterburner`))

(event `self.ReceiveTick`
  (params (DeltaSeconds :type "Float (single-precision)"))
  (`parent.ReceiveTick` DeltaSeconds))

(event `self.SetGear`
  (params (Value :type "Float (double-precision)"))
  ;[1 1 1] Sets Landing Gear Position
  (`self.RetractFrontWheel` Value)
  (`self.RetractRearLWheel` Value)
  (`self.RetractRearRWheel` Value))

(event `RetractFrontWheel`
  (params (Value :type "Float (double-precision)"))
  ;[1 1 1] Sets Front Gear Position
  (set `/Game/VigilanteMovement/Vehicles/West_Fighter_F35B/BPA_West_Fighter_F35B.FrontWheelRetract` Value (`self.AnimInstance`)))

(event `RetractRearLWheel`
  (params (Value :type "Float (double-precision)"))
  ;[1 1 1] Sets Rear Gears Position
  (set `/Game/VigilanteMovement/Vehicles/West_Fighter_F35B/BPA_West_Fighter_F35B.RearWheelLRetract` Value (`self.AnimInstance`)))

(event `RetractRearRWheel`
  (params (Value :type "Float (double-precision)"))
  ;[1 1 1] Sets Rear Gears Position
  (set `/Game/VigilanteMovement/Vehicles/West_Fighter_F35B/BPA_West_Fighter_F35B.RearWheelRRetract` Value (`self.AnimInstance`)))

(event `self.SetYaw`
  (params (Value :type "Float (double-precision)"))
  (bind _returnvalue (* Value -1.0))
  (bind _returnvalue_2 (`KismetMathLibrary.MapRangeClamped` _returnvalue -1.0 1.0 -10.0 10.0))
  ;[1 1 1] Sets Yaw on Rudders and Pilot Pedals
  (set `/Game/VigilanteMovement/Vehicles/West_Fighter_F35B/BPA_West_Fighter_F35B.RuddersAngle` (`KismetMathLibrary.MapRangeClamped` _returnvalue -1.0 1.0 -45.0 45.0) (`self.AnimInstance`))
  (set `/Game/VigilanteMovement/Vehicles/West_Fighter_F35B/BPA_West_Fighter_F35B.PedalLAngle` _returnvalue_2 (`self.AnimInstance`))
  (set `/Game/VigilanteMovement/Vehicles/West_Fighter_F35B/BPA_West_Fighter_F35B.PedalRAngle` _returnvalue_2 (`self.AnimInstance`)))

(event `self.SetRoll`
  (params (Value :type "Float (double-precision)"))
  (bind _returnvalue (* Value -1.0))
  ;[1 1 1] Set Roll on Ailerons and Pilot Stick
  (bind _output_get (set `/Game/VigilanteMovement/Vehicles/West_Fighter_F35B/BPA_West_Fighter_F35B.FlapsOuterLAngle` (`KismetMathLibrary.MapRangeClamped` _returnvalue -1.0 1.0 -60.0 60.0) (`self.AnimInstance`)))
  (set `/Game/VigilanteMovement/Vehicles/West_Fighter_F35B/BPA_West_Fighter_F35B.FlapsOuterRAngle` (* _output_get -1.0) (`self.AnimInstance`))
  (set `/Game/VigilanteMovement/Vehicles/West_Fighter_F35B/BPA_West_Fighter_F35B.CenterStickRoll` (`KismetMathLibrary.MapRangeClamped` (* _returnvalue -1.0) -1.0 1.0 -25.0 25.0) (`self.AnimInstance`)))

(event `self.SetPitch`
  (params (Pitch :type "Float (double-precision)"))
  ;[1 1 1] Sets Pitch on Stabilizers and Pilot Stick
  (bind _output_get (set `/Game/VigilanteMovement/Vehicles/West_Fighter_F35B/BPA_West_Fighter_F35B.StabilizerLAngle` (`KismetMathLibrary.MapRangeClamped` (* Pitch -1.0) -1.0 1.0 -30.0 30.0) (`self.AnimInstance`)))
  (set `/Game/VigilanteMovement/Vehicles/West_Fighter_F35B/BPA_West_Fighter_F35B.StabilizerRAngle` _output_get (`self.AnimInstance`))
  (set `/Game/VigilanteMovement/Vehicles/West_Fighter_F35B/BPA_West_Fighter_F35B.CenterStickPitch` (`KismetMathLibrary.MapRangeClamped` Pitch -1.0 1.0 -25.0 25.0) (`self.AnimInstance`)))

(event `self.SetThrottle`
  ;[1 1 1] Sets Throttle on Exhausts and Pilot Left Hand Lever
  (set `/Game/VigilanteMovement/Vehicles/West_Fighter_F35B/BPA_West_Fighter_F35B.ThrottlePosition` (`KismetMathLibrary.MapRangeClamped` (`self.Throttle`) 0.0 1.0 -5.0 5.0) (`self.AnimInstance`))
  (`|ExecutionSequence`
    (:`then_0`
      (if (not (`self.isAfterburnerActive`))
        (`self.SetExhaustNozzles` (`KismetMathLibrary.MapRangeClamped` (`self.Throttle`) 0.0 1.0 1.0 0.6))))
    (:`then_1`
      (if (`self.isVTOLActive`)
        (set `/Game/VigilanteMovement/Vehicles/West_Fighter_F35B/BPA_West_Fighter_F35B.FanVelocity` (* (`self.Throttle`) 1000.0) (`self.AnimInstance`))
        (else
          (set `/Game/VigilanteMovement/Vehicles/West_Fighter_F35B/BPA_West_Fighter_F35B.FanVelocity` 0.0 (`self.AnimInstance`)))))))

(event `SetExhaustNozzles`
  (params (Value :type "Float (double-precision)"))
  ;[1 1 1] Sets Exhaust Nozzles Size
  (bind _output_get (set `/Game/VigilanteMovement/Vehicles/West_Fighter_F35B/BPA_West_Fighter_F35B.ExhaustNozzles` Value (`self.AnimInstance`)))
  (bind _returnvalue (`KismetMathLibrary.MapRangeClamped` _output_get 0.0 1.0 0.2 0.3))
  (`NiagaraComponent.SetVariableVec3` (`self.NS_Jet`) "JetScale" (`KismetMathLibrary.MakeVector` (`KismetMathLibrary.MapRangeClamped` _output_get 0.0 1.0 0.25 0.8) _returnvalue _returnvalue))
  (`NiagaraComponent.SetVariableVec3` (`self.NS_Jet`) "JetRingsScale" (`KismetMathLibrary.MakeVector` 12.0 12.0 (`KismetMathLibrary.MapRangeClamped` _output_get 0.0 1.0 6.0 13.0)))
  (`FXSystemComponent.SetFloatParameter` (`self.NS_Jet`) "Opacity divide" (`KismetMathLibrary.MapRangeClamped` _output_get 0.0 1.0 2.0 0.8)))

(event `self.SetCanopy`
  (params (Value :type "Float (double-precision)"))
  ;[1 1 1] Sets Canopy Position
  (set `/Game/VigilanteMovement/Vehicles/West_Fighter_F35B/BPA_West_Fighter_F35B.Canopy` (* (`KismetMathLibrary.MapRangeClamped` Value 0.0 1.0 0.0 45.0) -1.0) (`self.AnimInstance`)))

(event `self.SetRefuel`
  (params (Value :type "Float (double-precision)"))
  ;[1 1 1] Sets Refuel
  (set `/Game/VigilanteMovement/Vehicles/West_Fighter_F35B/BPA_West_Fighter_F35B.Refuel` Value (`self.AnimInstance`)))

(event `self.SetBombBay`
  (params (Value :type "Float (double-precision)"))
  ;[1 1 1] Sets BombBay Shafts
  (set `/Game/VigilanteMovement/Vehicles/West_Fighter_F35B/BPA_West_Fighter_F35B.BombBay` (`KismetMathLibrary.MapRangeClamped` Value 0.0 1.0 0.0 90.0) (`self.AnimInstance`)))

(event `self.SetVTOLRatio`
  (params (Value :type "Float (double-precision)"))
  ;[1 1 1] VTOL Update
  (bind _output_get (set `/Game/VigilanteMovement/Vehicles/West_Fighter_F35B/BPA_West_Fighter_F35B.VTOLAngle` Value (`self.AnimInstance`)))
  (if (> _output_get 0.0)
    (if (not (`self.isVTOLActive`))
      (set `self.isVTOLActive` true)
      (`self.OpenFanShafts`))
    (elif (`self.isVTOLActive`)
      (`self.CloseFanShafts`))))

(event `OpenFanShafts`
  ;[1 1 1] Open Closes VTOL Fan Shafts
  (bind (_direction _cu_smooth_simplecurve) (`Timeline|FanShafts` :!label _label)
    (:`Update`
      (set `/Game/VigilanteMovement/Vehicles/West_Fighter_F35B/BPA_West_Fighter_F35B.VTOLShaftsPosition` _cu_smooth_simplecurve (`self.AnimInstance`)))
    (:`Finished`
      (if (`|EnumEquality` _direction "Backward")
        (set `self.isVTOLActive` false)))))

(event `CloseFanShafts`
  ;[1 1 1] Open Closes VTOL Fan Shafts
  (goto _label :!via `Reverse`))

(event `self.SetAfterburner`
  (bind _isafterburneractive (`self.isAfterburnerActive`))
  ;[1 1 1] Activates Afterburner VFX and Exhaust size
  (`ActorComponent.SetActive` (`self.NS_Jet`) _isafterburneractive true)
  (if _isafterburneractive
    (`self.SetExhaustNozzles` 1.0)
    (else
      (`self.SetExhaustNozzles` 0.6))))

(fn `UpdateDust`
  (if (`self.ShowDust`)
    (`NiagaraComponent.SetVariableFloat` (`self.DownwardDust`) "AirSpeed" (* (* (`self.Throttle`) (`self.DustMultiplicator`)) (- 1.0 (`self.VTOLRatio`))))
    (`NiagaraComponent.SetVariableFloat` (`self.DownwardDustVTOLFront`) "PropSpeed" (* (* (`self.Throttle`) (`self.VTOLDustFrontMultiplicator`)) (`self.VTOLRatio`)))
    (`NiagaraComponent.SetVariableFloat` (`self.DownwardDustVTOLRear`) "PropSpeed" (* (* (`self.Throttle`) (`self.VTOLDustRearMultiplicator`)) (`self.VTOLRatio`)))
    (else
      (`NiagaraComponent.SetVariableFloat` (`self.DownwardDust`) "AirSpeed" 0.0)
      (`NiagaraComponent.SetVariableFloat` (`self.DownwardDustVTOLFront`) "PropSpeed" 0.0)
      (`NiagaraComponent.SetVariableFloat` (`self.DownwardDustVTOLRear`) "AirSpeed" 0.0))))

(fn `UserConstructionScript`
  (`parent.UserConstructionScript`))